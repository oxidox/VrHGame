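; Doll actor that plays a staged disappearing and relocating sequence each time its Playerseen event fires.
; A SeenCounter picks the stage: the first sighting plays a turn-to-run animation, hides the skeletal mesh, teleports it and shows a standing pose.
; Later sightings swap Stand components and move through preset transforms.
; A separate showinwall event reveals the third pose, which the final sighting hides after a short delay.
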(event Custom|Playerseen
  (Development|PrintString "Hello")
  (if (== (Variables|Default|GetSeenCounter) 0)
    (Utilities|FlowControl|DoOnce false
      (:Completed
        (Components|Animation|PlayAnimation (Variables|Default|GetSkeletalMesh) "/Game/MoreModels/Girl/Mixamo/Running/Turn_To_Running_Anim.Turn_To_Running_Anim" false)
        (Utilities|FlowControl|Delay 2.26)
        (Rendering|SetVisibility (Variables|Default|GetSkeletalMesh) false false)
        (Transformation|SetActorTransform (Variables|Default|GetPos1))
        (Rendering|SetVisibility (Variables|Default|GetStand1) true false)
        (Variables|Default|SetSeenCounter (+ (Variables|Default|GetSeenCounter) 1))))
    (elif (== (Variables|Default|GetSeenCounter) 1)
      (Rendering|SetVisibility (Variables|Default|GetStand1) false false)
      (Transformation|SetActorTransform (Variables|Default|Getpos%202))
      (Rendering|SetVisibility (Variables|Default|GetStand2) true false)
      (Variables|Default|SetSeenCounter (+ (Variables|Default|GetSeenCounter) 1))
      (elif (== (Variables|Default|GetSeenCounter) 2)
        (Rendering|SetVisibility (Variables|Default|GetStand2) false false)
        (Transformation|SetActorTransform (Variables|Default|Getpos%203))
        (Variables|Default|SetSeenCounter (+ (Variables|Default|GetSeenCounter) 1))
        (elif (== (Variables|Default|GetSeenCounter) 3)
          (Utilities|FlowControl|Delay 0.5)
          (Rendering|SetVisibility (Variables|Default|GetStand3) false false))))))

(event Custom|showinwall
  (Rendering|SetVisibility (Variables|Default|GetStand3) true false))

(fn ConstructionScript)