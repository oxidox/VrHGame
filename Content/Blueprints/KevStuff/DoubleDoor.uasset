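; DoubleDoor Blueprint that swings two door halves in response to its Shut flag, which nothing in this graph sets.
; From BeginPlay, Delay loops poll Shut every 0.2 seconds instead of reacting to events.
; When Shut becomes true, LSphere and RSphere snap 90 degrees in opposite directions, then rotate back when it clears.
; The graph handles only one such cycle, as it never returns to the first wait.
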(event EventBeginPlay
  (if (Variables|Default|GetShut?) :!label _label
    (Utilities|FlowControl|Sequence
      (:then_0
        (Transformation|AddLocalRotation (Variables|Default|GetL%20Sphere) "0,-90.000000, 0" false false)
        (if (Variables|Default|GetShut?) :!label _label_2
          (Utilities|FlowControl|Delay 0.2)
          (goto _label_2)
          (else
            (Utilities|FlowControl|Sequence
              (:then_0
                (Transformation|AddLocalRotation (Variables|Default|GetL%20Sphere) "0,90.000000, 0" false false))
              (:then_1
                (Transformation|AddLocalRotation (Variables|Default|GetR%20Sphere) "0,-90.000000, 0" false false))))))
      (:then_1
        (Transformation|AddLocalRotation (Variables|Default|GetR%20Sphere) "0,90.000000, 0" false false)))
    (else
      (Utilities|FlowControl|Delay 0.2)
      (goto _label))))

(fn ConstructionScript)